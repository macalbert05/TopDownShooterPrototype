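; ShootingEnemy is an enemy Blueprint that fires a projectile at the player when the player pawn enters its RadarTrigger.
; The overlap passes the player's capsule position and velocity through Attack to ShootPlayer, which spawns a ShootingEnemyProjectile ahead of the Body.
; Aim leads the target a fixed distance along its movement, and the unnormalized offset becomes bullet velocity, so speed scales with distance.
; The close-range AttackTrigger detects the player but takes no action.
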(event `Attack`
  (params (PlayerLocation :type "Vector Structure") (PlayerVelocity :type "Vector Structure"))
  (`self.ShootPlayer` PlayerLocation PlayerVelocity))

(event `self.RadarTrigger.OnComponentBeginOverlap`
  (params (OverlappedComponent :type "PrimitiveComponent Object Reference") (OtherActor :type "Actor Object Reference") (OtherComp :type "PrimitiveComponent Object Reference") (OtherBodyIndex :type Integer) (bFromSweep :type Boolean) (SweepResult :type "HitResult Structure (by ref)"))
  ;[1 1 1] If player is nearby
  (bind _asplayer_pawn (cast `PlayerPawn` OtherActor))
  (`/Engine/EditorBlueprintResources/StandardMacros.IsValid` _asplayer_pawn
    (:`Is Valid`
      (bind _playercapsulecomponent (`PlayerPawn.PlayerCapsuleComponent` _asplayer_pawn))
      (bind _returnvalue (`PrimitiveComponent.GetPhysicsLinearVelocity` _playercapsulecomponent "None"))
      (`self.Attack` (`SceneComponent.K2_GetComponentLocation` _playercapsulecomponent) _returnvalue))))

(event `self.AttackTrigger.OnComponentBeginOverlap`
  (params (OverlappedComponent :type "PrimitiveComponent Object Reference") (OtherActor :type "Actor Object Reference") (OtherComp :type "PrimitiveComponent Object Reference") (OtherBodyIndex :type Integer) (bFromSweep :type Boolean) (SweepResult :type "HitResult Structure (by ref)"))
  ;[1 1 1] If player is very close
  (bind _asplayer_pawn (cast `PlayerPawn` OtherActor))
  (`/Engine/EditorBlueprintResources/StandardMacros.IsValid` _asplayer_pawn))

(fn `ShootPlayer`
  (params (targetLocation :type "Vector Structure") (targetVelocity :type "Vector Structure"))
  (bind _body (`self.Body`))
  (bind _returnvalue (+ (`SceneComponent.K2_GetComponentLocation` _body) (* (`SceneComponent.GetForwardVector` _body) (`self.spawnDistance`))))
  (bind _returnvalue_2 (`|SpawnActorFromClass` "/Game/Blueprints/EnemiesBP/ShootingEnemyProjectile.ShootingEnemyProjectile_C" (`KismetMathLibrary.MakeTransform` _returnvalue) "Undefined" "OverrideRootScale" null null))
  (`PrimitiveComponent.SetPhysicsLinearVelocity` (`/Game/Blueprints/EnemiesBP/ShootingEnemyProjectile.Bullet` _returnvalue_2) (- (+ targetLocation (* (`KismetMathLibrary.Normal` targetVelocity) (`self.unitsAhead`))) _returnvalue) false "None"))

(fn `UserConstructionScript`
  (`parent.UserConstructionScript`))