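; Enemy spawner actor that spawns waves of enemies around its mesh, starting shortly after BeginPlay.
; SpawnEnemy stores type, amount and cycle count in EnemyQuery, then a looping timer runs ExecuteQuery until the cycles finish.
; Each enemy gets a random same-height point within a scale-dependent range, validated by a line trace from the spawner.
; Blocked points retry a limited number of times before that spawn is skipped.
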(event `self.ReceiveBeginPlay`
  (`KismetSystemLibrary.Delay` 3.0)
  (`self.SpawnEnemy` 1 2 5 1.5))

(event `AddEnemy`)

(event `SpawnEnemy`
  (params (Type :type Integer) (Amount :type Integer) (SpawnCycle :type Integer) (SpawnSpeed :type "Float (double-precision)"))
  (`self.SpawnEnemies` Type Amount SpawnCycle SpawnSpeed))

(fn `ExecuteQuery`
  (for _ (range 1 (+ (`|GetArrayItem` (`self.EnemyQuery`) 1) 1))
    (bind (_newvalidlocation _foundvalidlocation) (`self.GetValidLocation`))
    (if _foundvalidlocation
      (`|SpawnActorFromClass` (`|GetArrayItem` (`self.ListOfEnemies`) (`|GetArrayItem` (`self.EnemyQuery`))) (`KismetMathLibrary.MakeTransform` _newvalidlocation) "Undefined" "OverrideRootScale" null null)))
  (bind _result (`/Engine/EditorBlueprintResources/StandardMacros.IncrementInt` (`self.enemiesSpawned`))
    (:`  `
      (if (>= _result (`|GetArrayItem` (`self.EnemyQuery`) 2))
        (`KismetSystemLibrary.K2_ClearAndInvalidateTimerHandle` (`self.TimerHandle`))
        (`KismetArrayLibrary.Array_Clear` (`self.EnemyQuery`))
        (set `self.enemiesSpawned` 0)))))

(fn `GetRandomLocation`
  (returns (NewRandomPosition :type "Vector Structure"))
  (bind (_returnvalue_x _returnvalue_y _returnvalue_z) (`KismetMathLibrary.BreakVector` (`SceneComponent.K2_GetComponentLocation` (`self.SpawnerMesh`))))
  (bind _returnvalue (* (`KismetMathLibrary.VSize` (`SceneComponent.K2_GetComponentScale` (`self.SpawnerMesh`))) (`self.maxSpawnDistance`)))
  (bind _returnvalue_2 (* _returnvalue -1.0))
  (return (`KismetMathLibrary.MakeVector` (+ _returnvalue_x (`KismetMathLibrary.RandomFloatInRange` _returnvalue_2 _returnvalue)) (+ _returnvalue_y (`KismetMathLibrary.RandomFloatInRange` _returnvalue_2 _returnvalue)) _returnvalue_z)))

(fn `GetValidLocation`
  (returns (NewValidLocation :type "Vector Structure") (foundValidLocation :type Boolean))
  (locals (isSearching :type Boolean :default true) (validLocation :type "Vector Structure") (confirmValidLocation :type Boolean :default false))
  (while (`local.isSearching`)
    (if (>= (`self.searchCycle`) 5)
      ;[1 1 1] IF no empty location to spawn...
      (set `local.isSearching` false)
      (set `self.searchCycle` 0)
      (set `local.confirmValidLocation` false)
      (else
        (bind _newrandomposition (`self.GetRandomLocation`))
        (bind _isobstructed (`self.PerimeterCheck` (`SceneComponent.K2_GetComponentLocation` (`self.SpawnerMesh`)) _newrandomposition))
        (bind _output_get (set `local.isSearching` _isobstructed))
        (if _output_get
          (`/Engine/EditorBlueprintResources/StandardMacros.IncrementInt` (`self.searchCycle`))
          (else
            (set `local.validLocation` _newrandomposition)
            (set `local.confirmValidLocation` true))))))
  (set `local.isSearching` true)
  (return (`local.validLocation`) (`local.confirmValidLocation`)))

(fn `PerimeterCheck`
  (params (StartPosition :type "Vector Structure") (PositionToSpawn :type "Vector Structure"))
  (returns (isObstructed :type Boolean))
  (bind (_outhit _returnvalue) (`KismetSystemLibrary.LineTraceSingleByProfile` StartPosition PositionToSpawn))
  (return _returnvalue))

(fn `SpawnEnemies`
  (params (Type :type Integer) (Amount :type Integer) (SpawnCycle :type Integer) (SpawnSpeed :type "Float (double-precision)"))
  (bind _enemyquery (`self.EnemyQuery`))
  (`KismetArrayLibrary.Array_Clear` _enemyquery)
  (`KismetArrayLibrary.Array_Add` _enemyquery Type)
  (`KismetArrayLibrary.Array_Add` _enemyquery Amount)
  (`KismetArrayLibrary.Array_Add` _enemyquery SpawnCycle)
  (bind _returnvalue (`KismetSystemLibrary.K2_SetTimer` null "ExecuteQuery" SpawnSpeed true))
  (set `self.TimerHandle` _returnvalue))

(fn `UserConstructionScript`)