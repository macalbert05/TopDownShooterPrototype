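; SuicideEnemy is an enemy Blueprint that launches its physics body at the player.
; An Attack event or a player entering RadarTrigger calls TacklePlayer, which sets Body velocity once to the offset toward the target scaled by TackleSpeed.
; The target velocity is passed in but unused, so the tackle does not lead the player.
; AttackTrigger detects a very close player but takes no action yet.
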(event `Attack`
  (params (playerLocation :type "Vector Structure") (playerVelocity :type "Vector Structure"))
  (`self.TacklePlayer` playerLocation playerVelocity))

(event `self.RadarTrigger.OnComponentBeginOverlap`
  (params (OverlappedComponent :type "PrimitiveComponent Object Reference") (OtherActor :type "Actor Object Reference") (OtherComp :type "PrimitiveComponent Object Reference") (OtherBodyIndex :type Integer) (bFromSweep :type Boolean) (SweepResult :type "HitResult Structure (by ref)"))
  ;[1 1 1] If player is nearby
  (bind _asplayer_pawn (cast `PlayerPawn` OtherActor))
  (`/Engine/EditorBlueprintResources/StandardMacros.IsValid` _asplayer_pawn
    (:`Is Valid`
      (bind _playercapsulecomponent (`PlayerPawn.PlayerCapsuleComponent` _asplayer_pawn))
      (bind _returnvalue (`PrimitiveComponent.GetPhysicsLinearVelocity` _playercapsulecomponent "None"))
      (`self.TacklePlayer` (`SceneComponent.K2_GetComponentLocation` _playercapsulecomponent) _returnvalue))))

(event `self.AttackTrigger.OnComponentBeginOverlap`
  (params (OverlappedComponent :type "PrimitiveComponent Object Reference") (OtherActor :type "Actor Object Reference") (OtherComp :type "PrimitiveComponent Object Reference") (OtherBodyIndex :type Integer) (bFromSweep :type Boolean) (SweepResult :type "HitResult Structure (by ref)"))
  ;[1 1 1] If player is very close
  (bind _asplayer_pawn (cast `PlayerPawn` OtherActor))
  (`/Engine/EditorBlueprintResources/StandardMacros.IsValid` _asplayer_pawn))

(fn `TacklePlayer`
  (params (targetLocation :type "Vector Structure") (targetVelocity :type "Vector Structure"))
  (`PrimitiveComponent.SetPhysicsLinearVelocity` (`self.Body`) (* (- targetLocation (`SceneComponent.K2_GetComponentLocation` (`self.Body`))) (`self.tackleSpeed`)) false "None"))

(fn `UserConstructionScript`
  (`parent.UserConstructionScript`))