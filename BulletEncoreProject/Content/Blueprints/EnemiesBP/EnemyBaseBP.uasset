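; Base enemy Blueprint that runs altitude control every tick and exposes events to chase or evade the player's pawn, or destroy itself.
; Chase, Evade and AltitudeControl are called but not defined here.
; An unwired Patrol uses recursive, retry-limited line traces to pick a random horizontal destination, re-rolling the offset after the trace.
; A looping timer then drives the physics body toward it by velocity until arrival.
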(event `self.ReceiveBeginPlay`
  (if (`self.isMoving`)
    _))

(event `self.ReceiveTick`
  (params (DeltaSeconds :type "Float (single-precision)"))
  (`self.AltitudeControl`))

(event `ChasePlayer`
  (`self.Chase` (`self.K2_GetActorLocation` (`Controller.K2_GetPawn` (`GameplayStatics.GetPlayerController` 0)))))

(event `EvadePlayer`
  (`self.Evade` (`self.K2_GetActorLocation` (`Controller.K2_GetPawn` (`GameplayStatics.GetPlayerController` 0)))))

(event `Destroy`
  (`self.K2_DestroyActor`))

(fn `FindRandomDestination`
  (returns (NewDestination :type "Vector Structure"))
  (locals (nextDestination :type "Vector Structure"))
  (bind _searchradius (`self.searchRadius`))
  (bind _returnvalue (`SceneComponent.K2_GetComponentLocation` (`self.Body`)))
  (bind _returnvalue_2 (* _searchradius -1.0))
  (bind _returnvalue_3 (+ _returnvalue (`KismetMathLibrary.MakeVector` (`KismetMathLibrary.RandomFloatInRange` _returnvalue_2 _searchradius) (`KismetMathLibrary.RandomFloatInRange` _returnvalue_2 _searchradius))))
  (if (>= (`self.searchAttempt`) 5)
    (set `local.nextDestination` _returnvalue)
    (return (`local.nextDestination`))
    (else
      (bind (_outhit _returnvalue_4) (`KismetSystemLibrary.LineTraceSingleByProfile` :`Start` _returnvalue :`End` _returnvalue_3 :`DrawDebugType` "ForDuration"))
      (if _returnvalue_4
        (`/Engine/EditorBlueprintResources/StandardMacros.IncrementInt` (`self.searchAttempt`)
          (:`  `
            (`self.FindRandomDestination`)))
        (else
          (set `local.nextDestination` _returnvalue_3)
          (set `self.searchAttempt` 0)
          (return (`local.nextDestination`)))))))

(fn `Moving`
  (bind _returnvalue (- (`self.targetDestination`) (`SceneComponent.K2_GetComponentLocation` (`self.Body`))))
  (set `self.isMoving` true)
  (if (<= (`KismetMathLibrary.VSize` _returnvalue) 5.0)
    (`KismetSystemLibrary.K2_ClearAndInvalidateTimerHandle` (`self.TimerHandle`))
    (set `self.isMoving` false)
    (`PrimitiveComponent.SetPhysicsLinearVelocity` (`self.Body`) (0.0 0.0 0.0) false "None")
    (else
      (`PrimitiveComponent.SetPhysicsLinearVelocity` (`self.Body`) (* (`KismetMathLibrary.Normal` _returnvalue) (`self.speed`)) false "None"))))

(fn `Patrol`
  (bind _newdestination (`self.FindRandomDestination`))
  (set `self.targetDestination` _newdestination)
  (bind _returnvalue (`KismetSystemLibrary.K2_SetTimer` null "Moving" (`self.frameCycle`) true))
  (set `self.TimerHandle` _returnvalue))

(fn `UserConstructionScript`)