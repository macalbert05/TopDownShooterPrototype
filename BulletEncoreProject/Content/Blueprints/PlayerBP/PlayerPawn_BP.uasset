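; Player pawn Blueprint that extends parent shooting and damage logic with an aiming laser, health bar and HUD updates.
; Each tick a line trace places the laser beam's end, with the source offset by movement input to counter lag.
; Projectile hits on capsule or hitbox apply damage, destroy the projectile and show a health bar that fades after a timeout.
; Begin play and firing push ammo and lives to the game mode's HUD.
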(event `self.ReceiveBeginPlay`
  (bind _returnvalue (`|CreateWidget` "/Game/UI/PlayerHealthBar.PlayerHealthBar_C" (`GameplayStatics.GetPlayerController` 0)))
  (`UserWidget.AddToViewport` _returnvalue 0)
  (set `self.PlayerHealthWidget` _returnvalue)
  (`self.UpdateHealthBarValues`)
  (`self.UpdatePlayerHUDStats`))

(event `self.ReceiveTick`
  (params (DeltaSeconds :type "Float (single-precision)"))
  (`self.SpawnLaserFromLocationTowardsAimDirection` (`SceneComponent.K2_GetComponentLocation` (`self.ShootFromPoint`)))
  (`self.UpdateHealthBarVisibility` DeltaSeconds))

(event `UpdateHealthBarValues`
  (bind _playerhealthwidget (`self.PlayerHealthWidget`))
  (bind (_playerhealth_numberoflives _playerhealth_maxhealth _playerhealth_currenthealth) (break `PlayerHealthInfo` (`self.PlayerHealth`)))
  (bind _playerhealthwidget_2 (`self.PlayerHealthWidget`))
  (`/Engine/EditorBlueprintResources/StandardMacros.IsValid` _playerhealthwidget_2
    (:`Is Valid`
      (`/Game/UI/PlayerHealthBar.UpdateHealth` _playerhealthwidget_2 _playerhealth_currenthealth _playerhealth_maxhealth)
      (if (and (< (`Widget.GetRenderOpacity` (`/Game/UI/PlayerHealthBar.HealthBar` _playerhealthwidget)) 1.0) (!= (`UserWidget.IsPlayingAnimation` _playerhealthwidget) true))
        (`/Game/UI/PlayerHealthBar.FadeInHealthBar` _playerhealthwidget))
      (set `self.TimeSpentShowingHealthBar` 0.0))))

(event `self.FireShotFromCurrentGun`
  (`parent.FireShotFromCurrentGun`)
  (`self.UpdatePlayerHUDStats`))

(event `self.ReloadCurrentGun`
  (`parent.ReloadCurrentGun`))

(event `self.PlayerCapsuleComponent.OnComponentHit`
  (params (HitComponent :type "PrimitiveComponent Object Reference") (OtherActor :type "Actor Object Reference") (OtherComp :type "PrimitiveComponent Object Reference") (NormalImpulse :type "Vector Structure") (Hit :type "HitResult Structure (by ref)"))
  (`self.OnContactWithDamagingObject` OtherActor))

(event `self.HitBox.OnComponentHit`
  (params (HitComponent :type "PrimitiveComponent Object Reference") (OtherActor :type "Actor Object Reference") (OtherComp :type "PrimitiveComponent Object Reference") (NormalImpulse :type "Vector Structure") (Hit :type "HitResult Structure (by ref)"))
  (`self.OnContactWithDamagingObject` OtherActor))

(event `TakeDamage`
  (`self.OnTakeDamage` 1.0)
  (`self.UpdateHealthBarValues`))

(event `OnContactWithDamagingObject`
  (params (OtherActorRef :type "Actor Object Reference"))
  (`/Engine/EditorBlueprintResources/StandardMacros.IsValid` OtherActorRef
    (:`Is Valid`
      (bind _asbase_projectile_class (cast `BaseProjectileClass` OtherActorRef))
      (bind _returnvalue (`BaseProjectileClass.GetBulletData` _asbase_projectile_class))
      (bind _returnvalue_2 (`self.OnTakeDamage` (`KismetMathLibrary.Conv_IntToDouble` (`.damage` (break `BulletData` _returnvalue)))))
      (`KismetSystemLibrary.PrintString` (`KismetStringLibrary.Concat_StrStr` "Player Took Damage" (`KismetStringLibrary.Conv_DoubleToString` _returnvalue_2)) true true (struct :`R` 1.0 :`G` 0.451018 :`A` 1.0))
      (`self.K2_DestroyActor` OtherActorRef))))

(fn `OnTakeDamage`
  (params (damage :type "Float (double-precision)"))
  (returns (ReturnValue :type "Float (double-precision)"))
  (bind _returnvalue (`parent.OnTakeDamage` damage))
  (`self.UpdateHealthBarValues`)
  (return _returnvalue))

(fn `SpawnLaserFromLocationTowardsAimDirection`
  (params (SpawnLocation :type "Vector Structure"))
  (locals (LaserEndLocation :type "Vector Structure") (defaultLengthOfLaser :type "Float (double-precision)" :default 1200.0) (LaserStartLocation :type "Vector Structure"))
  (bind _returnvalue (+ (* (`self.GetCurrentAimDirection`) (`local.defaultLengthOfLaser`)) (`local.LaserStartLocation`)))
  (set `local.LaserStartLocation` SpawnLocation)
  (bind _outhit (`KismetSystemLibrary.LineTraceSingle` (`local.LaserStartLocation`) _returnvalue "TraceTypeQuery1"))
  (bind (_bblockinghit _binitialoverlap _time _distance _location) (`GameplayStatics.BreakHitResult` _outhit))
  (if _bblockinghit
    (set `local.LaserEndLocation` _location)
    (else
      (set `local.LaserEndLocation` _returnvalue)))
  (`ParticleSystemComponent.SetBeamSourcePoint` (`self.LaserSystem`) 0 (+ (`local.LaserStartLocation`) (* (`self.GetMovementAxisInput`) 5.0)) 0)
  (`ParticleSystemComponent.SetBeamTargetPoint` (`self.LaserSystem`) 0 (`local.LaserEndLocation`) 0))

(fn `UpdateHealthBarVisibility`
  (params (deltaTime :type "Float (double-precision)"))
  (bind _playerhealthwidget (`self.PlayerHealthWidget`))
  (if (and (> (`Widget.GetRenderOpacity` (`/Game/UI/PlayerHealthBar.HealthBar` _playerhealthwidget)) 0.0) (!= (`UserWidget.IsPlayingAnimation` _playerhealthwidget) true))
    (set `self.TimeSpentShowingHealthBar` (+ deltaTime (`self.TimeSpentShowingHealthBar`)))
    (if (> (`self.TimeSpentShowingHealthBar`) (`self.LifeTimeOfHealthBar`))
      (`/Engine/EditorBlueprintResources/StandardMacros.DoOnce` false :!label _label
        (:`Completed`
          (`/Game/UI/PlayerHealthBar.FadeOutHealthBar` (`self.PlayerHealthWidget`))))
      (else
        (goto _label :!via `Reset`)))))

(fn `UpdatePlayerHUDStats`
  (locals (PlayerHUDRef :type "/Game/UI/PlayerGameplayHUD Object Reference") (CurrentGunData :type "GunData Structure"))
  (bind (_rateoffire _bisspreadfire _currentclipcount _maxclipcount) (break `GunData` (`local.CurrentGunData`)))
  (`|ExecutionSequence`
    (:`then_0`
      (bind _asgame_mode_default (cast `/Game/Blueprints/GameMode/GameModeDefault` (`GameplayStatics.GetGameMode`)))
      (set `local.PlayerHUDRef` (`/Game/Blueprints/GameMode/GameModeDefault.PlayerGameplayHUD` _asgame_mode_default))
      (set `local.CurrentGunData` (`self.GetCurrentGunData`)))
    (:`then_1`
      (`/Game/UI/PlayerGameplayHUD.UpdateAmmoClipData` (`local.PlayerHUDRef`) _currentclipcount _maxclipcount)
      (`/Game/UI/PlayerGameplayHUD.UpdateCurrentAmmo` (`local.PlayerHUDRef`) (`.currentAmmoCount` (break `GunData` (`local.CurrentGunData`))))
      (`/Game/UI/PlayerGameplayHUD.UpdateMaxAmmo` (`local.PlayerHUDRef`) (`.maxAmmoCount` (break `GunData` (`local.CurrentGunData`))))
      (`/Game/UI/PlayerGameplayHUD.UpdateLives` (`local.PlayerHUDRef`) (`.numberOfLives` (break `PlayerHealthInfo` (`self.PlayerHealth`)))))))

(fn `UserConstructionScript`)