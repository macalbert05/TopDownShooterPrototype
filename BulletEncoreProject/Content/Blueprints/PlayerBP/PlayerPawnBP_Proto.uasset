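; PlayerPawnBP_Proto is a prototype player pawn that projects a laser beam along the current aim direction.
; Every Tick, it line-traces on Visibility from ShootFromPoint to a default length, ending the beam at any blocking hit.
; It then sets the source and target points of the LaserSystem beam emitter.
; The source point is nudged by movement input to counter visual lag while moving.
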(event `self.ReceiveBeginPlay`)

(event `self.ReceiveTick`
  (params (DeltaSeconds :type "Float (single-precision)"))
  (`self.SpawnLaserFromLocationTowardsAimDirection` (`SceneComponent.K2_GetComponentLocation` (`self.ShootFromPoint`))))

(fn `SpawnLaserFromLocationTowardsAimDirection`
  (params (SpawnLocation :type "Vector Structure"))
  (locals (LaserEndLocation :type "Vector Structure") (defaultLengthOfLaser :type "Float (double-precision)" :default 1200.0) (LaserStartLocation :type "Vector Structure"))
  (bind _returnvalue (+ (* (`self.GetCurrentAimDirection`) (`local.defaultLengthOfLaser`)) (`local.LaserStartLocation`)))
  (set `local.LaserStartLocation` SpawnLocation)
  (bind _outhit (`KismetSystemLibrary.LineTraceSingle` (`local.LaserStartLocation`) _returnvalue "TraceTypeQuery1"))
  (bind (_bblockinghit _binitialoverlap _time _distance _location) (`GameplayStatics.BreakHitResult` _outhit))
  (if _bblockinghit
    (set `local.LaserEndLocation` _location)
    (else
      (set `local.LaserEndLocation` _returnvalue)))
  (`ParticleSystemComponent.SetBeamSourcePoint` (`self.LaserSystem`) 0 (+ (`local.LaserStartLocation`) (* (`self.GetMovementAxisInput`) 5.0)) 0)
  (`ParticleSystemComponent.SetBeamTargetPoint` (`self.LaserSystem`) 0 (`local.LaserEndLocation`) 0))

(fn `UserConstructionScript`)