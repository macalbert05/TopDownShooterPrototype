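; Obstacle generator that builds a 40-by-40 grid of obstacle actors scaled to a Floor and raises a random subset.
; When IsActive, BeginPlay spawns the grid, picks ActiveIndices and starts a looping timer that steps their meshes upward until a height limit.
; ShuffleObstacles starts the descend timer, then immediately re-randomizes and starts the ascend timer, without waiting for descent.
; Up and Down keys trigger either motion for testing.
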(event `self.ReceiveBeginPlay`
  ;[1 1 1] Turn obstacle ON at Start??
  (if (`self.isActive`)
    (`self.EnableInput` (`GameplayStatics.GetPlayerController` 0))
    (`self.GenerateObstacleBoard`)
    (`self.RandomizeTiles`)
    (bind _returnvalue (`KismetSystemLibrary.K2_SetTimer` null "AscendTiles" (`self.timeCycle`) true))
    (set `self.timerHandler` _returnvalue)))

(event `ShuffleObstacles`
  (`KismetSystemLibrary.K2_SetTimer` null "DescendTiles" (`self.timeCycle`) true)
  (`self.RandomizeTiles`)
  (`KismetSystemLibrary.K2_SetTimer` null "AscendTiles" (`self.timeCycle`) true))

(event `Key|Up`
  (params (Key :type "Key Structure"))
  ;[1 1 1] For testing
  (:`Pressed`
    (`KismetSystemLibrary.K2_SetTimer` null "AscendTiles" (`self.timeCycle`) true)))

(event `Key|Down`
  (params (Key :type "Key Structure"))
  ;[1 1 1] For testing
  (:`Pressed`
    (`KismetSystemLibrary.K2_SetTimer` null "DescendTiles" (`self.timeCycle`) true)))

(fn `AscendTiles`
  (locals (ActiveObstacleRef :type "Array of /Game/Blueprints/ObstacleObject Object Reference"))
  (if (>= (`self.heightAdjust`) (`self.maxRaiseDistance`))
    (`KismetSystemLibrary.K2_PauseTimerHandle` (`self.timerHandler`))
    (else
      (set `self.heightAdjust` (+ (`self.heightAdjust`) (`self.distancePerFrame`)))
      (for _array_element (`self.ActiveIndices`)
        (bind _mesh (`/Game/Blueprints/ObstacleObject.Mesh` (`|GetArrayItem` (`self.ObstacleList`) _array_element)))
        (bind (_returnvalue_x _returnvalue_y _returnvalue_z) (`KismetMathLibrary.BreakVector` (`SceneComponent.K2_GetComponentLocation` _mesh)))
        (`SceneComponent.K2_SetWorldLocation` _mesh (`KismetMathLibrary.MakeVector` _returnvalue_x _returnvalue_y (+ _returnvalue_z (`self.heightAdjust`))) false false)))))

(fn `DescendTiles`
  (locals (ActiveObstacleRef :type "Array of /Game/Blueprints/ObstacleObject Object Reference"))
  (if (<= (`self.heightAdjust`) 0.0)
    (`KismetSystemLibrary.K2_PauseTimerHandle` (`self.timerHandler`))
    (else
      (for _array_element (`self.ActiveIndices`)
        (bind _output_get (set `self.heightAdjust` (- (`self.heightAdjust`) (`self.distancePerFrame`))))
        (bind _mesh (`/Game/Blueprints/ObstacleObject.Mesh` (`|GetArrayItem` (`self.ObstacleList`) _array_element)))
        (bind (_returnvalue_x _returnvalue_y _returnvalue_z) (`KismetMathLibrary.BreakVector` (`SceneComponent.K2_GetComponentLocation` _mesh)))
        (`SceneComponent.K2_SetWorldLocation` _mesh (`KismetMathLibrary.MakeVector` _returnvalue_x _returnvalue_y (- _returnvalue_z _output_get)) false false)))))

(fn `GenerateObstacleBoard`
  (bind (_spacerunits_x _spacerunits_y) (`KismetMathLibrary.BreakVector` (`self.spacerUnits`)))
  (bind _spacerunits_x_2 (`KismetMathLibrary.BreakVector` (`self.spacerUnits`)))
  (bind (_spacervector_x _spacervector_y _spacervector_z) (`KismetMathLibrary.BreakVector` (`self.spacerVector`)))
  (bind (_scaleratio_x _scaleratio_y _scaleratio_z) (`KismetMathLibrary.BreakVector` (`self.scaleRatio`)))
  (bind (_scaleratio_x_2 _scaleratio_y_2 _scaleratio_z_2) (`KismetMathLibrary.BreakVector` (`self.scaleRatio`)))
  (bind _floor (`self.Floor`))
  (bind (_spacervector_x_2 _spacervector_y_2) (`KismetMathLibrary.BreakVector` (`self.spacerVector`)))
  (bind _startspawnposition_x (`KismetMathLibrary.BreakVector` (`self.startSpawnPosition`)))
  (bind (_spacervector_x_3 _spacervector_y_3 _spacervector_z_2) (`KismetMathLibrary.BreakVector` (`self.spacerVector`)))
  (bind (_spacerunits_x_3 _spacerunits_y_2 _spacerunits_z) (`KismetMathLibrary.BreakVector` (`self.spacerUnits`)))
  (bind _scaleratio_x_3 (`KismetMathLibrary.BreakVector` (`self.scaleRatio`)))
  (bind (_returnvalue_x _returnvalue_y) (`KismetMathLibrary.BreakVector` (/ (`SceneComponent.K2_GetComponentScale` _floor) 40.0)))
  (set `self.spacerVector` (`self.startSpawnPosition`))
  (bind _output_get (set `self.scaleRatio` (`KismetMathLibrary.MakeVector` _returnvalue_x _returnvalue_y (`self.obstacleHeightScale`))))
  (set `self.spacerUnits` (`KismetMathLibrary.MakeVector` (* (.x _output_get) _spacerunits_x_3) (* (.y _output_get) _spacerunits_y_2) _spacerunits_z))
  (for _index (range 1 1601)
    (if (== (mod _index 40) 0)
      (bind _returnvalue (+ (`SceneComponent.K2_GetComponentLocation` _floor) (`KismetMathLibrary.MakeVector` (* _spacervector_x_3 (.x _output_get)) (* _spacervector_y_3 (.y _output_get)) _spacervector_z_2)))
      (bind _returnvalue_2 (`|SpawnActorFromClass` "/Game/Blueprints/ObstacleObject.ObstacleObject_C" (`KismetMathLibrary.MakeTransform` _returnvalue (struct) (`KismetMathLibrary.MakeVector` _scaleratio_x _scaleratio_y _scaleratio_z)) "Undefined" "OverrideRootScale" null null))
      (set `self.spacerVector` (`KismetMathLibrary.MakeVector` (* _startspawnposition_x _scaleratio_x_3) (+ _spacervector_y_2 _spacerunits_y)))
      (`KismetArrayLibrary.Array_Add` (`self.ObstacleList`) _returnvalue_2)
      (else
        (bind _returnvalue_3 (`|SpawnActorFromClass` "/Game/Blueprints/ObstacleObject.ObstacleObject_C" (`KismetMathLibrary.MakeTransform` _returnvalue (struct) (`KismetMathLibrary.MakeVector` _scaleratio_x_2 _scaleratio_y_2 _scaleratio_z_2)) "Undefined" "OverrideRootScale" null null))
        (set `self.spacerVector` (`KismetMathLibrary.MakeVector` (+ _spacervector_x _spacerunits_x_2) _spacervector_y _spacervector_z))
        (`KismetArrayLibrary.Array_Add` (`self.ObstacleList`) _returnvalue_3)))))

(fn `RandomizeTiles`
  (`KismetArrayLibrary.Array_Clear` (`self.ActiveIndices`))
  (for _ (range 1 (+ (`self.numActiveObstacles`) 1))
    (`KismetArrayLibrary.Array_AddUnique` (`self.ActiveIndices`) (`KismetMathLibrary.RandomIntegerInRange` 0 (- (`KismetArrayLibrary.Array_Length` (`self.ObstacleList`)) 1)))))

(fn `UserConstructionScript`)