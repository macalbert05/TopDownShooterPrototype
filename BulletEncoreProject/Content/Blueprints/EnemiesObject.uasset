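; Enemy actor that homes in on the player's pawn using a physics-simulated body with gravity disabled.
; A looping timer started on BeginPlay calls ChasePlayer by name, setting the body's X/Y velocity along the normalized direction to the pawn, scaled by Speed.
; EvadePlayer mirrors this with negated Speed to flee, but nothing in this Blueprint calls it.
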(event `self.ReceiveBeginPlay`
  (`KismetSystemLibrary.K2_SetTimer` null "ChasePlayer" 0.1 true))

(fn `ChasePlayer`
  (bind _returnvalue (`Controller.K2_GetPawn` (`GameplayStatics.GetPlayerController` 0)))
  (bind (_returnvalue_x _returnvalue_y) (`KismetMathLibrary.BreakVector` (* (`KismetMathLibrary.Normal` (- (`self.K2_GetActorLocation` _returnvalue) (`SceneComponent.K2_GetComponentLocation` (`self.EnemyBody`)))) (`self.speed`))))
  (`/Engine/EditorBlueprintResources/StandardMacros.IsValid` _returnvalue
    (:`Is Valid`
      (`PrimitiveComponent.SetPhysicsLinearVelocity` (`self.EnemyBody`) (`KismetMathLibrary.MakeVector` _returnvalue_x _returnvalue_y) false "None"))))

(fn `EvadePlayer`
  (bind _returnvalue (`Controller.K2_GetPawn` (`GameplayStatics.GetPlayerController` 0)))
  (bind (_returnvalue_x _returnvalue_y) (`KismetMathLibrary.BreakVector` (* (`KismetMathLibrary.Normal` (- (`self.K2_GetActorLocation` _returnvalue) (`SceneComponent.K2_GetComponentLocation` (`self.EnemyBody`)))) (* (`self.speed`) -1.0))))
  (`/Engine/EditorBlueprintResources/StandardMacros.IsValid` _returnvalue
    (:`Is Valid`
      (`PrimitiveComponent.SetPhysicsLinearVelocity` (`self.EnemyBody`) (`KismetMathLibrary.MakeVector` _returnvalue_x _returnvalue_y) false "None"))))

(fn `UserConstructionScript`
  (bind _enemybody (`self.EnemyBody`))
  (`PrimitiveComponent.SetSimulatePhysics` _enemybody true)
  (`PrimitiveComponent.SetEnableGravity` _enemybody false))