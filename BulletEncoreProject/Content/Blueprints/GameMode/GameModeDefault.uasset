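; Default game mode Blueprint that puts the player's gameplay HUD on screen when play begins.
; BeginPlay calls DisplayInGameUI, which creates the PlayerGameplayHUD widget, stores a reference and adds it to the viewport.
; A CustomCursor event can hide the system cursor and show a MouseCursor widget instead, but its only call is disconnected, so it never runs here.
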(event `self.ReceiveBeginPlay`
  (`self.DisplayInGameUI`))

(event `DisplayInGameUI`
  (bind _returnvalue (`|CreateWidget` "/Game/UI/PlayerGameplayHUD.PlayerGameplayHUD_C"))
  (set `self.PlayerGameplayHUD` _returnvalue)
  (`UserWidget.AddToViewport` _returnvalue 0))

(event `CustomCursor`
  (set `PlayerController.bShowMouseCursor` false (`GameplayStatics.GetPlayerController` 0))
  (bind _returnvalue (`|CreateWidget` "/Game/UI/MouseCursor.MouseCursor_C"))
  (bind _output_get (set `self.MouseCursorRef` _returnvalue))
  (`UserWidget.AddToViewport` _output_get 0))

(fn `UserConstructionScript`)