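; ObstacleGenerator spawns a 40x40 grid of obstacle cubes scaled from its Floor and raises or lowers a random subset of them.
; RandomizeTiles picks the active indices, then MoveTiles starts a looping timer on MovingLoop, which steps their shared height between min and max.
; Activate, Deactivate and Shuffle events drive it; shuffling lowers the cubes, then re-randomizes and raises them.
; Up and Down keys trigger shuffle and deactivate for testing.
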(event `self.ReceiveBeginPlay`
  ;[1 1 1] For testing
  (`self.EnableInput` (`GameplayStatics.GetPlayerController` 0))
  (`self.GenerateObstacleBoard`)
  ;[1 1 1] Turn obstacle ON at Start??
  (if (`self.isActiveFromStart`)
    (`self.RandomizeTiles`)
    (`self.MoveTiles` true)))

(event `Key|Up`
  (params (Key :type "Key Structure"))
  ;[1 1 1] For testing
  (:`Pressed`
    (`self.ShuffleObstacles`)))

(event `ShuffleObstacles`
  ;[1 1 1] Call this event to reset & randomize the obstacles
  (set `self.isShuffling` true)
  (`self.MoveTiles` false))

(event `Key|Down`
  (params (Key :type "Key Structure"))
  ;[1 1 1] For testing
  (:`Pressed`
    (`self.DeactivateObstacles`)))

(event `DeactivateObstacles`
  ;[1 1 1] Call this event to turn off & lower the obstacles
  (`self.MoveTiles` false))

(event `ActivateObstacles`
  ;[1 1 1] Call this event to turn on the obstacles after deactivation
  (`self.RandomizeTiles`)
  (`self.MoveTiles` true))

(fn `GenerateObstacleBoard`
  (bind (_spacerunits_x _spacerunits_y) (`KismetMathLibrary.BreakVector` (`self.spacerUnits`)))
  (bind _spacerunits_x_2 (`KismetMathLibrary.BreakVector` (`self.spacerUnits`)))
  (bind (_spacervector_x _spacervector_y _spacervector_z) (`KismetMathLibrary.BreakVector` (`self.spacerVector`)))
  (bind _floor (`self.Floor`))
  (bind (_spacervector_x_2 _spacervector_y_2) (`KismetMathLibrary.BreakVector` (`self.spacerVector`)))
  (bind _startspawnpositionconst_x (`KismetMathLibrary.BreakVector` (`self.startSpawnPositionConst`)))
  (bind (_returnvalue_x _returnvalue_y) (`KismetMathLibrary.BreakVector` (/ (`SceneComponent.K2_GetComponentScale` _floor) 40.0)))
  (bind (_returnvalue_x_2 _returnvalue_y_2 _returnvalue_z) (`KismetMathLibrary.BreakVector` (`SceneComponent.K2_GetComponentLocation` (`/Game/Blueprints/ObstacleBP/ObstacleObject.Mesh` (`|GetArrayItem` (`self.ObstacleList`))))))
  (set `self.spacerVector` (`self.startSpawnPositionConst`))
  (set `self.scaleRatio` (`KismetMathLibrary.MakeVector` _returnvalue_x _returnvalue_y (`self.obstacleHeightScale`)))
  (for _index (range 1 1601)
    ;[1 1 1] Create cube obstacle & store ref
    (bind _returnvalue (`|SpawnActorFromClass` "/Game/Blueprints/ObstacleBP/ObstacleObject.ObstacleObject_C" (`KismetMathLibrary.MakeTransform` (+ (`self.spacerVector`) (`SceneComponent.K2_GetComponentLocation` _floor)) (struct) (`self.scaleRatio`)) "Undefined" "OverrideRootScale" null null))
    (`KismetArrayLibrary.Array_Add` (`self.ObstacleList`) _returnvalue)
    (if (== (mod _index 40) 0)
      (set `self.spacerVector` (`KismetMathLibrary.MakeVector` _startspawnpositionconst_x (+ _spacervector_y_2 _spacerunits_y)))
      (else
        (set `self.spacerVector` (`KismetMathLibrary.MakeVector` (+ _spacervector_x _spacerunits_x_2) _spacervector_y _spacervector_z)))))
  ;[1 1 1 1 12] Get the z-position of the first cube to be used as a reference when calculating the moving positions of all the cubes (generalized all cubes's height as the same height)
  (set `self.initialHeight_guide` _returnvalue_z))

(fn `MoveTiles`
  (params (`moveTileUp?` :type Boolean))
  (bind _timerhandler (`self.timerHandler`))
  ;[1 1 1] IF timer already exist, then reset Timer
  (if (`KismetSystemLibrary.K2_IsValidTimerHandle` _timerhandler)
    (`KismetSystemLibrary.K2_ClearAndInvalidateTimerHandle` _timerhandler))
  (bind _output_get (set `self.isGoingUp` `moveTileUp?`))
  ;[1 1 1 1 12] Going up or down? True = UP // False = DOWN
  (if _output_get
    ;[1 1 1] IF false starts loop
    (if (not (>= (`self.currentHeight`) (`self.maxHeight`)))
      (set `self.directionModifier` 1.0)
      ;[1 1 1] Shifting/Moving loop
      (bind _returnvalue (`KismetSystemLibrary.K2_SetTimer` null "MovingLoop" (`self.timeCycle`) true :!label _label))
      (set `self.timerHandler` _returnvalue))
    (elif (not (<= (`self.currentHeight`) (`self.minHeight`)))
      (set `self.directionModifier` -1.0)
      (goto _label))))

(fn `MovingLoop`
  (locals (ActiveObstacleRef :type "Array of /Game/Blueprints/ObstacleBP/ObstacleObject Object Reference"))
  (if (`self.isGoingUp`)
    ;[1 1 1] Is it at max or min height yet?
    (if (>= (`self.currentHeight`) (`self.maxHeight`))
      (`KismetSystemLibrary.K2_ClearAndInvalidateTimerHandle` (`self.timerHandler`))
      (if (`self.isShuffling`)
        (set `self.isShuffling` false))
      (else
        ;[1 1 1] Up or Down control
        (set `self.currentHeight` (+ (`self.currentHeight`) (* (`self.distancePerCycle`) (`self.directionModifier`))) :!label _label)
        ;[1 1 1] Animating/(Ascending/Descending) Shifting cycle
        (for _array_element (`self.ActiveIndices`)
          (bind _mesh (`/Game/Blueprints/ObstacleBP/ObstacleObject.Mesh` (`|GetArrayItem` (`self.ObstacleList`) _array_element)))
          (bind (_returnvalue_x _returnvalue_y) (`KismetMathLibrary.BreakVector` (`SceneComponent.K2_GetComponentLocation` _mesh)))
          (`SceneComponent.K2_SetWorldLocation` _mesh (`KismetMathLibrary.MakeVector` _returnvalue_x _returnvalue_y (+ (`self.initialHeight_guide`) (`self.currentHeight`))) false false))))
    (elif (<= (`self.currentHeight`) (`self.minHeight`))
      (`KismetSystemLibrary.K2_ClearAndInvalidateTimerHandle` (`self.timerHandler`))
      (if (`self.isShuffling`)
        (`self.RandomizeTiles`)
        (`self.MoveTiles` true))
      (else
        (goto _label)))))

(fn `RandomizeTiles`
  (`KismetArrayLibrary.Array_Clear` (`self.ActiveIndices`))
  (for _ (range 1 (+ (`self.numOfActiveObstacles`) 1))
    (`KismetArrayLibrary.Array_AddUnique` (`self.ActiveIndices`) (`KismetMathLibrary.RandomIntegerInRange` 0 (- (`KismetArrayLibrary.Array_Length` (`self.ObstacleList`)) 1)))))

(fn `UserConstructionScript`)