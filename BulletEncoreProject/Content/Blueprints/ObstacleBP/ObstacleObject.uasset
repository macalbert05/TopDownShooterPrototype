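; Obstacle actor Blueprint that displays a selectable static mesh.
; On BeginPlay it picks the mesh from MeshList using MeshIndex clamped to the list bounds, and a SetMesh event can replace it with any given mesh.
; The construction script creates a dynamic instance of ObstacleMat on the mesh's first material slot and stores it in MaterialRef.
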(event `self.ReceiveBeginPlay`
  (bind _meshlist (`self.MeshList`))
  (`StaticMeshComponent.SetStaticMesh` (`self.Mesh`) (`|GetArrayItem` _meshlist (`KismetMathLibrary.Clamp` (`self.MeshIndex`) 0 (- (`KismetArrayLibrary.Array_Length` _meshlist) 1)))))

(event `SetMesh`
  (params (StaticMesh :type "StaticMesh Object Reference"))
  (`StaticMeshComponent.SetStaticMesh` (`self.Mesh`) StaticMesh))

(fn `UserConstructionScript`
  (bind _returnvalue (`PrimitiveComponent.CreateDynamicMaterialInstance` (`self.Mesh`) 0 "/Game/Material/ObstacleMat.ObstacleMat" "None"))
  (set `self.MaterialRef` _returnvalue))