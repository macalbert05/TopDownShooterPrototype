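; Enemy spawner actor that periodically creates batches of enemies around itself.
; On BeginPlay it starts a looping timer that calls SpawnEnemies every SpawnTimeCycle seconds.
; Each cycle spawns NumEnemiesSpawn actors of EnemiesObject at random X/Y offsets around SpawnerMesh, at the mesh's height.
; The spread scales with the length of the mesh's world scale vector, so resizing the mesh changes the spawn area.
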(event `self.ReceiveBeginPlay`
  (`KismetSystemLibrary.K2_SetTimer` null "SpawnEnemies" (`self.spawnTimeCycle`) true))

(fn `SpawnEnemies`
  (bind (_returnvalue_x _returnvalue_y _returnvalue_z) (`KismetMathLibrary.BreakVector` (`SceneComponent.K2_GetComponentLocation` (`self.SpawnerMesh`))))
  (bind _returnvalue (* (`KismetMathLibrary.VSize` (`SceneComponent.K2_GetComponentScale` (`self.SpawnerMesh`))) 200.0))
  (bind _returnvalue_2 (* _returnvalue -1.0))
  (for _ (range 1 (+ (`self.NumEnemiesSpawn`) 1))
    (`|SpawnActorFromClass` "/Game/Blueprints/EnemiesObject.EnemiesObject_C" (`KismetMathLibrary.MakeTransform` (`KismetMathLibrary.MakeVector` (+ _returnvalue_x (`KismetMathLibrary.RandomFloatInRange` _returnvalue_2 _returnvalue)) (+ _returnvalue_y (`KismetMathLibrary.RandomFloatInRange` _returnvalue_2 _returnvalue)) _returnvalue_z)) "Undefined" "OverrideRootScale" null null)))

(fn `UserConstructionScript`)