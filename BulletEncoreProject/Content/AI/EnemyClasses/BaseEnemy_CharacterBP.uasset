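; Base enemy character Blueprint that takes damage when struck by projectiles.
; Hits on the capsule and HitBox components both route to OnContactWithBullet, which casts to BaseProjectileClass and reads the bullet's damage.
; That damage goes through OnTakeDamage to the parent implementation, then a debug message prints and the projectile is destroyed.
; Firing and reloading simply forward to the parent class.
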(event `self.FireShotFromCurrentGun`
  (params (bulletSpawnPoint :type "Vector Structure (by ref)"))
  (`parent.FireShotFromCurrentGun` bulletSpawnPoint))

(event `self.ReloadCurrentGun`
  (`parent.ReloadCurrentGun`))

(event `self.CapsuleComponent.OnComponentHit`
  (params (HitComponent :type "PrimitiveComponent Object Reference") (OtherActor :type "Actor Object Reference") (OtherComp :type "PrimitiveComponent Object Reference") (NormalImpulse :type "Vector Structure") (Hit :type "HitResult Structure (by ref)"))
  (`self.OnContactWithBullet` OtherActor))

(event `self.HitBox.OnComponentHit`
  (params (HitComponent :type "PrimitiveComponent Object Reference") (OtherActor :type "Actor Object Reference") (OtherComp :type "PrimitiveComponent Object Reference") (NormalImpulse :type "Vector Structure") (Hit :type "HitResult Structure (by ref)"))
  (`self.OnContactWithBullet` OtherActor))

(event `OnContactWithBullet`
  (params (ActorRef :type "Actor Object Reference"))
  (`/Engine/EditorBlueprintResources/StandardMacros.IsValid` ActorRef
    (:`Is Valid`
      (bind _asbase_projectile_class (cast `BaseProjectileClass` ActorRef))
      (bind _returnvalue (`BaseProjectileClass.GetBulletData` _asbase_projectile_class))
      (bind _returnvalue_2 (`self.OnTakeDamage` (`KismetMathLibrary.Conv_IntToDouble` (`.damage` (break `BulletData` _returnvalue)))))
      (`KismetSystemLibrary.PrintString` (`KismetStringLibrary.Concat_StrStr` "Enemy Took Damage" (`KismetStringLibrary.Conv_DoubleToString` _returnvalue_2)) true true (struct :`R` 1.0 :`G` 0.451018 :`A` 1.0))
      (`self.K2_DestroyActor` ActorRef))))

(fn `OnTakeDamage`
  (params (damage :type "Float (double-precision)"))
  (returns (ReturnValue :type "Float (double-precision)"))
  (bind _returnvalue (`parent.OnTakeDamage` damage))
  (return _returnvalue))

(fn `UserConstructionScript`)